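; Doors is an automatic two-panel sliding door driven by a trigger volume.
; Any overlap plays the Door_Driver timeline, whose separate left and right tracks lerp each panel's relative location between stored start and end vectors.
; When an overlap ends, the timeline reverses after a short delay to slide the panels back, without checking whether other actors remain inside.
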(event OnComponentEndOverlap(TriggerVolume)
  (params (OverlappedComponent :type Primitive%20Component%20Object%20Reference) (OtherActor :type Actor%20Object%20Reference) (OtherComp :type Primitive%20Component%20Object%20Reference) (OtherBodyIndex :type Integer))
  (Utilities|FlowControl|Delay 0.5)
  (bind (_direction _door_l_a _door_l_b _door_r_a _door_r_b) (Timeline|Door_Driver Reverse)
    (:Update
      (Transformation|SetRelativeLocation (Variables|Default|GetDoor_Left-B) (Math|Vector|Lerp(Vector) (Variables|DoorSetup|GetDoor_L-B%20Start) (Variables|Default|GetDoor_L-B%20End) _door_l_b) false false)
      (Transformation|SetRelativeLocation (Variables|Default|GetDoor_Right-B) (Math|Vector|Lerp(Vector) (Variables|DoorSetup|GetDoor_R-B%20Sart) (Variables|Default|GetDoor_R-B%20End) _door_r_b) false false))))

(event OnComponentBeginOverlap(TriggerVolume)
  (params (OverlappedComponent :type Primitive%20Component%20Object%20Reference) (OtherActor :type Actor%20Object%20Reference) (OtherComp :type Primitive%20Component%20Object%20Reference) (OtherBodyIndex :type Integer) (bFromSweep :type Boolean) (SweepResult :type Hit%20Result%20Structure%20%28by%20ref%29))
  (bind (_direction _door_l_a _door_l_b _door_r_a _door_r_b) (Timeline|Door_Driver Play)
    (:Update
      (Transformation|SetRelativeLocation (Variables|Default|GetDoor_Left-B) (Math|Vector|Lerp(Vector) (Variables|DoorSetup|GetDoor_L-B%20Start) (Variables|Default|GetDoor_L-B%20End) _door_l_b) false false)
      (Transformation|SetRelativeLocation (Variables|Default|GetDoor_Right-B) (Math|Vector|Lerp(Vector) (Variables|DoorSetup|GetDoor_R-B%20Sart) (Variables|Default|GetDoor_R-B%20End) _door_r_b) false false))))

(fn ConstructionScript)