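; SplinePipe-A is a construction-script Blueprint that builds a deformable sci-fi pipe along a spline.
; It divides the spline length by Spacing and adds a collidable spline mesh component for each step, using the Pipe_Deformable mesh and SciPipes material.
; Each segment takes world-space positions and directions at its two distances along the spline, with tangents scaled by TangentScale, and is created with manual attachment.
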(fn ConstructionScript
  (bind _splinepipe_a (Variables|Default|GetSplinePipe-A))
  (bind _spacing (Variables|Default|GetSpacing))
  (bind _tangent_scale (Variables|Default|GetTangent%20Scale))
  (for _index (range 0 (.ReturnValue (Math|Float|Division(WholeandRemainder) (Spline|GetSplineLength _splinepipe_a) _spacing)))
    (bind _returnvalue (AddComponent|AddSplineMeshComponent true))
    (Collision|SetCollisionEnabled _returnvalue "QueryAndPhysics")
    (Components|StaticMesh|SetStaticMesh _returnvalue "/Game/Stasis_Pack/Meshes/Splines/Pipe_Deformable.Pipe_Deformable")
    (Rendering|Material|SetMaterial _returnvalue 0 "/Game/Stasis_Pack/Materials/Sci-Pipes_MAT.Sci-Pipes_MAT")
    (SplineMesh|SetStartandEnd _returnvalue (Class|SplineComponent|GetWorldLocationatDistanceAlongSpline _splinepipe_a (* _index _spacing)) (* (Class|SplineComponent|GetWorldDirectionatDistanceAlongSpline _splinepipe_a (* _index _spacing)) _tangent_scale) (Class|SplineComponent|GetWorldLocationatDistanceAlongSpline _splinepipe_a (+ (* _index _spacing) _spacing)) (* (Class|SplineComponent|GetWorldDirectionatDistanceAlongSpline _splinepipe_a (+ (* _index _spacing) _spacing)) _tangent_scale) :!class /Script/Engine.SplineMeshComponent)))