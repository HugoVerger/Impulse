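; Conditional sliding door Blueprint that opens when something overlaps its trigger volume, provided it is unlocked.
; On BeginPlay it compares DoorTest against DoorLevel; if high enough, it clears LockedDoor and turns both lock-state lights green.
; Overlap begin plays a timeline that lerps the left and right door panels between start and end positions; overlap end reverses it after a short delay.
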(event OnComponentEndOverlap(TriggerVolume)
  (params (OverlappedComponent :type Primitive%20Component%20Object%20Reference) (OtherActor :type Actor%20Object%20Reference) (OtherComp :type Primitive%20Component%20Object%20Reference) (OtherBodyIndex :type Integer))
  ;[1 1 1] Door Openning and Closing
  (if (not (Variables|Default|GetLockedDoor))
    (Utilities|FlowControl|Delay 0.5)
    (bind (_direction _door_l_a _door_l_b _door_r_a _door_r_b) (Timeline|Door_Driver Reverse)
      (:Update
        (Transformation|SetRelativeLocation (Variables|Default|GetDoor_Left-B) (Math|Vector|Lerp(Vector) (Variables|DoorSetup|GetDoor_L-B%20Start) (Variables|Default|GetDoor_L-B%20End) _door_l_b) false false)
        (Transformation|SetRelativeLocation (Variables|Default|GetDoor_Right-B) (Math|Vector|Lerp(Vector) (Variables|DoorSetup|GetDoor_R-B%20Sart) (Variables|Default|GetDoor_R-B%20End) _door_r_b) false false)))))

(event OnComponentBeginOverlap(TriggerVolume)
  (params (OverlappedComponent :type Primitive%20Component%20Object%20Reference) (OtherActor :type Actor%20Object%20Reference) (OtherComp :type Primitive%20Component%20Object%20Reference) (OtherBodyIndex :type Integer) (bFromSweep :type Boolean) (SweepResult :type Hit%20Result%20Structure%20%28by%20ref%29))
  ;[1 1 1] Door Openning and Closing
  (if (not (Variables|Default|GetLockedDoor))
    (bind (_direction _door_l_a _door_l_b _door_r_a _door_r_b) (Timeline|Door_Driver Play)
      (:Update
        (Transformation|SetRelativeLocation (Variables|Default|GetDoor_Left-B) (Math|Vector|Lerp(Vector) (Variables|DoorSetup|GetDoor_L-B%20Start) (Variables|Default|GetDoor_L-B%20End) _door_l_b) false false)
        (Transformation|SetRelativeLocation (Variables|Default|GetDoor_Right-B) (Math|Vector|Lerp(Vector) (Variables|DoorSetup|GetDoor_R-B%20Sart) (Variables|Default|GetDoor_R-B%20End) _door_r_b) false false)))))

(event EventBeginPlay
  ;[1 1 1] Light Conditional Coloration
  (if (>= (Variables|Default|GetDoorTest) (Variables|Default|GetDoorLevel))
    (Variables|Default|SetLockedDoor false)
    (Rendering|Components|Light|SetLightColor (Variables|Default|GetLockStateLight) "(R=0.035294,G=0.933333,B=0.000000,A=1.000000)" true)
    (Rendering|Components|Light|SetLightColor (Variables|Default|GetLockStateLight2) "(R=0.035294,G=0.933333,B=0.000000,A=1.000000)" true)))

(fn ConstructionScript)