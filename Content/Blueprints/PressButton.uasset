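; A one-shot press button that, when the first-person character hits its cube, clears a blocking wall and moves another.
; The hit destroys WallBlocking, then starts moving WallToMove if valid; without a valid WallBlocking, neither happens.
; A timeline at a configurable play rate drives the target wall cube's relative location, scaled by Variation and masked by MovingAxis.
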(event OnComponentHit(Cube)
  (params (HitComponent :type Primitive%20Component%20Object%20Reference) (OtherActor :type Actor%20Object%20Reference) (OtherComp :type Primitive%20Component%20Object%20Reference) (NormalImpulse :type Vector :default "0, 0, 0") (Hit :type Hit%20Result%20Structure%20%28by%20ref%29))
  (bind _wallblocking (Variables|Default|GetWallBlocking))
  ;[1 1 1] Trigger on player detection
  (if (not (Variables|Default|GetHasBeenTriggered))
    (Utilities|Casting|CastToFirstPersonCharacter OtherActor)
    (Variables|Default|SetHasBeenTriggered true)
    (if (Utilities|IsValid _wallblocking)
      (Actor|DestroyActor _wallblocking)
      (if (Utilities|IsValid (Variables|Default|GetWallToMove))
        (CallFunction|StartMovingWall)))))

(event Custom|StartMovingWall
  ;[1 1 1] Moving Wall
  (Utilities|FlowControl|Sequence
    (:then_0
      (bind _movingtrack (Timeline|Moving PlayFromStart)
        (:Update
          (Transformation|SetRelativeLocation (Variables|/Game/Blueprints/DeathWall.DeathWall_C|GetCube (Variables|Default|GetWallToMove)) (* (Math|Vector|MakeVector (* _movingtrack (Variables|Default|GetVariation)) (* _movingtrack (Variables|Default|GetVariation)) (* _movingtrack (Variables|Default|GetVariation))) (Variables|Default|GetMovingAxis)) false false))))
    (:then_1
      (Components|Timeline|SetPlayRate (Variables|Default|GetMoving) (Variables|Default|GetPlayRate)))))

(fn ConstructionScript)