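; Small sliding door that opens for the first-person character while unlocked.
; Box trigger overlaps play and reverse the DoorPosition timeline, which drives the Cube's relative location, with a sound on opening only.
; BeginPlay clears LockedDoor and turns both lock-state lights green if DoorTest is at least DoorLevel.
; The lock is evaluated only once, at BeginPlay.
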(event OnComponentBeginOverlap(Box)
  (params (OverlappedComponent :type Primitive%20Component%20Object%20Reference) (OtherActor :type Actor%20Object%20Reference) (OtherComp :type Primitive%20Component%20Object%20Reference) (OtherBodyIndex :type Integer) (bFromSweep :type Boolean) (SweepResult :type Hit%20Result%20Structure%20%28by%20ref%29))
  ;[1 1 1] Door openning and Closing
  (if (not (Variables|Default|GetLockedDoor))
    (Utilities|Casting|CastToFirstPersonCharacter OtherActor)
    (Audio|PlaySoundatLocation "/Game/Sounds/DoorOpening.DoorOpening" (Transformation|GetActorLocation) "0, 0, 0" 0.8)
    (bind _doorslider (Timeline|DoorPosition Play)
      (:Update
        (Transformation|SetRelativeLocation (Variables|Default|GetCube) _doorslider false false)))))

(event OnComponentEndOverlap(Box)
  (params (OverlappedComponent :type Primitive%20Component%20Object%20Reference) (OtherActor :type Actor%20Object%20Reference) (OtherComp :type Primitive%20Component%20Object%20Reference) (OtherBodyIndex :type Integer))
  ;[1 1 1] Door openning and Closing
  (if (not (Variables|Default|GetLockedDoor))
    (Utilities|Casting|CastToFirstPersonCharacter OtherActor)
    (bind _doorslider (Timeline|DoorPosition Reverse)
      (:Update
        (Transformation|SetRelativeLocation (Variables|Default|GetCube) _doorslider false false)))))

(event EventBeginPlay
  ;[1 1 1] Light Conditional Coloration
  (if (>= (Variables|Default|GetDoorTest) (Variables|Default|GetDoorLevel))
    (Variables|Default|SetLockedDoor false)
    (Rendering|Components|Light|SetLightColor (Variables|Default|GetLockStateLight2) "(R=0.035294,G=0.933333,B=0.000000,A=1.000000)" true)
    (Rendering|Components|Light|SetLightColor (Variables|Default|GetLockStateLight) "(R=0.035294,G=0.933333,B=0.000000,A=1.000000)" true)))

(fn ConstructionScript)