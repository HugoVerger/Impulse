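; PressStressWall is a one-shot trigger actor that rearranges walls when the first-person character hits its cube.
; On that hit it destroys WallBlocking, starts moving WallToMove and reveals WallToSpawn, which is hidden without collision or tick at BeginPlay.
; The Moving timeline, sped by PlayRate, sets the moving wall cube's relative location from its track, scaled by Variation and masked by MovingAxis.
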(event OnComponentHit(Cube)
  (params (HitComponent :type Primitive%20Component%20Object%20Reference) (OtherActor :type Actor%20Object%20Reference) (OtherComp :type Primitive%20Component%20Object%20Reference) (NormalImpulse :type Vector :default "0, 0, 0") (Hit :type Hit%20Result%20Structure%20%28by%20ref%29))
  (bind _walltospawn (Variables|Default|GetWallToSpawn))
  (bind _wallblocking (Variables|Default|GetWallBlocking))
  ;[1 1 1] Player Detection
  (if (not (Variables|Default|GetHasBeenTriggered))
    (Utilities|Casting|CastToFirstPersonCharacter OtherActor)
    (Variables|Default|SetHasBeenTriggered true)
    (Utilities|FlowControl|Sequence
      (:then_0
        (if (Utilities|IsValid _wallblocking)
          (Actor|DestroyActor _wallblocking)))
      (:then_1
        (if (Utilities|IsValid (Variables|Default|GetWallToMove))
          (CallFunction|StartMovingWall)))
      (:then_2
        (if (Utilities|IsValid _walltospawn)
          (Rendering|SetActorHiddenInGame _walltospawn false)
          (Actor|Tick|SetActorTickEnabled _walltospawn true)
          (Collision|SetActorEnableCollision _walltospawn true))))))

(event Custom|StartMovingWall
  ;[1 1 1] Moving Wall
  (Utilities|FlowControl|Sequence
    (:then_0
      (bind _movingtrack (Timeline|Moving PlayFromStart)
        (:Update
          (Transformation|SetRelativeLocation (Variables|/Game/Blueprints/DeathWall.DeathWall_C|GetCube (Variables|Default|GetWallToMove)) (* (Math|Vector|MakeVector (* _movingtrack (Variables|Default|GetVariation)) (* _movingtrack (Variables|Default|GetVariation)) (* _movingtrack (Variables|Default|GetVariation))) (Variables|Default|GetMovingAxis)) false false))))
    (:then_1
      (Components|Timeline|SetPlayRate (Variables|Default|GetMoving) (Variables|Default|GetPlayRate)))))

(event EventBeginPlay
  (bind _walltospawn (Variables|Default|GetWallToSpawn))
  ;[1 1 1] Disable the WallToSpawn
  (if (Utilities|IsValid _walltospawn)
    (Rendering|SetActorHiddenInGame _walltospawn true)
    (Actor|Tick|SetActorTickEnabled _walltospawn)
    (Collision|SetActorEnableCollision _walltospawn false)))

(fn ConstructionScript)