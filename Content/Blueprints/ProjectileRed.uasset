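; Red projectile that destroys itself on impact and places a red force field where it hits a red zone.
; Hits on blue projectiles are ignored; other hits require a static mesh using the M_RedZone material, otherwise a debug message prints.
; Spawning destroys any existing ForceFieldRed, so only one exists at a time.
; A scene component added at the hit point anchors the field to the struck component, keeping world rotation and scale.
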(event Collision|EventHit
  (params (MyComp :type Primitive%20Component%20Object%20Reference) (Other :type Actor%20Object%20Reference) (OtherComp :type Primitive%20Component%20Object%20Reference) (bSelfMoved :type Boolean) (HitLocation :type Vector) (HitNormal :type Vector :default "0, 0, 0") (NormalImpulse :type Vector :default "0, 0, 0") (Hit :type Hit%20Result%20Structure%20%28by%20ref%29))
  (bind _returnvalue (Math|Transform|MakeTransform HitLocation))
  ;[1 1 1] Spawn ForceField and destroy projectile
  (Variables|Default|SetOtherActor Other)
  (Variables|Default|SetOtherComp OtherComp)
  (Actor|DestroyActor)
  (Utilities|Casting|CastToProjectileBlue (Variables|Default|GetOtherActor)
    (:CastFailed
      (bind _asstatic_mesh_component (Utilities|Casting|CastToStaticMeshComponent (Variables|Default|GetOtherComp))
        (:then
          (if (== (Rendering|Material|GetMaterial _asstatic_mesh_component 0) "/Game/Materials/M_RedZone.M_RedZone")
            (CallFunction|SpawnForceFieldRed _returnvalue)
            (bind _returnvalue_2 (AddComponent|AddSceneComponent (Variables|Default|GetOtherActor) false (Math|Transform|MakeTransform (Math|Transform|InverseTransformLocation (Class|KismetMathLibrary|ConvertTransformtoRelative _returnvalue (Transformation|GetWorldTransform (Variables|Default|GetOtherComp))) "0, 0, 0"))))
            (Transformation|AttachComponentToComponent _returnvalue_2 (Variables|Default|GetOtherComp) "None" "KeepRelative" "KeepWorld" "KeepWorld" false)
            (if (Utilities|IsValid (Variables|Default|GetNewForceFieldRed))
              (Transformation|AttachComponentToComponent (Variables|Default|GetNewForceFieldRed) _returnvalue_2 "None" "SnapToTarget" "KeepWorld" "KeepWorld" false))
            (else
              (Development|PrintString "Not on a Red Zone !" :!label _label))))
        (:CastFailed
          (goto _label))))))

(fn ConstructionScript)

(fn SpawnForceFieldRed
  (params (SpawnTransform :type Transform))
  (bind _outactors (Actor|GetAllActorsOfClass "/Game/Blueprints/ForceFieldRed.ForceFieldRed_C"))
  (Actor|DestroyActor _outactors)
  (bind _returnvalue (Game|SpawnActorfromClass "/Game/Blueprints/ForceFieldRed.ForceFieldRed_C" SpawnTransform "AlwaysSpawn" 0 0))
  (Variables|Default|SetNewForceFieldRed _returnvalue))