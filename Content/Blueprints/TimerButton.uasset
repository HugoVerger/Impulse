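; TimerButton is an interactable actor that starts or stops a timer on the first-person character.
; A Box overlap tracks whether a FirstPersonCharacter is inside the button's zone.
; The actor enables its own input on BeginPlay, so pressing Use inside the zone calls StartTimer, or StopTimer when IsEndButton is set, on the player character.
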(event OnComponentBeginOverlap(Box)
  (params (OverlappedComponent :type Primitive%20Component%20Object%20Reference) (OtherActor :type Actor%20Object%20Reference) (OtherComp :type Primitive%20Component%20Object%20Reference) (OtherBodyIndex :type Integer) (bFromSweep :type Boolean) (SweepResult :type Hit%20Result%20Structure%20%28by%20ref%29))
  ;[1 1 1] Player Zone Detection
  (Utilities|Casting|CastToFirstPersonCharacter OtherActor)
  (Variables|Default|SetIsPlayerInside true))

(event OnComponentEndOverlap(Box)
  (params (OverlappedComponent :type Primitive%20Component%20Object%20Reference) (OtherActor :type Actor%20Object%20Reference) (OtherComp :type Primitive%20Component%20Object%20Reference) (OtherBodyIndex :type Integer))
  ;[1 1 1] Player Zone Detection
  (Utilities|Casting|CastToFirstPersonCharacter OtherActor)
  (Variables|Default|SetIsPlayerInside false))

(event EventBeginPlay
  ;[1 1 1] Enabling input detection
  (Input|EnableInput (Game|GetPlayerController 0)))

(event Input|ActionEvents|InputActionUse
  (params (Key :type Key%20Structure :default "AnyKey"))
  ;[1 1 1] Button Pressing
  (:Pressed
    (if (Variables|Default|GetIsPlayerInside)
      (bind _asfirst_person_character (Utilities|Casting|CastToFirstPersonCharacter (Game|GetPlayerCharacter 0)))
      (if (Variables|Default|GetIsEndButton)
        (Default|StopTimer _asfirst_person_character)
        (else
          (Default|StartTimer _asfirst_person_character))))))

(fn ConstructionScript)