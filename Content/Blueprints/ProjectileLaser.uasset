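; Laser projectile that kills the first-person player on overlap and is destroyed when it hits something.
; Killing the player disables the laser's collision, then restarts the current level after a short delay.
; Overlapping a blue force field multiplies its velocity and a red one divides it by the same factor, with each change reversed on exit.
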(event OnComponentBeginOverlap(CollisionComponent)
  (params (OverlappedComponent :type Primitive%20Component%20Object%20Reference) (OtherActor :type Actor%20Object%20Reference) (OtherComp :type Primitive%20Component%20Object%20Reference) (OtherBodyIndex :type Integer) (bFromSweep :type Boolean) (SweepResult :type Hit%20Result%20Structure%20%28by%20ref%29))
  (bind _projectile (Variables|MyProjectile|GetProjectile))
  ;[1 1 1] Player and ForceField detection
  (bind _asfirst_person_character (Utilities|Casting|CastToFirstPersonCharacter OtherActor)
    (:then
      (Default|Kill _asfirst_person_character)
      (Collision|SetCollisionEnabled (Variables|MyProjectile|GetCollisionComponent) "NoCollision")
      (Utilities|FlowControl|Delay 0.5)
      (bind _returnvalue (Game|GetCurrentLevelName true))
      (Game|OpenLevel(byName) (Utilities|String|StringToName _returnvalue)))
    (:CastFailed
      (Utilities|Casting|CastToForceFieldBlue OtherActor
        (:then
          (Variables|/Script/Engine.MovementComponent|SetVelocity _projectile (* (Variables|/Script/Engine.MovementComponent|GetVelocity _projectile) 5)))
        (:CastFailed
          (Utilities|Casting|CastToForceFieldRed OtherActor)
          (Variables|/Script/Engine.MovementComponent|SetVelocity _projectile (/ (Variables|/Script/Engine.MovementComponent|GetVelocity _projectile) 5)))))))

(event OnComponentEndOverlap(CollisionComponent)
  (params (OverlappedComponent :type Primitive%20Component%20Object%20Reference) (OtherActor :type Actor%20Object%20Reference) (OtherComp :type Primitive%20Component%20Object%20Reference) (OtherBodyIndex :type Integer))
  (bind _projectile (Variables|MyProjectile|GetProjectile))
  ;[1 1 1] Player and ForceField detection
  (Utilities|Casting|CastToForceFieldBlue OtherActor
    (:then
      (Variables|/Script/Engine.MovementComponent|SetVelocity _projectile (/ (Variables|/Script/Engine.MovementComponent|GetVelocity _projectile) 5)))
    (:CastFailed
      (Utilities|Casting|CastToForceFieldRed OtherActor)
      (Variables|/Script/Engine.MovementComponent|SetVelocity _projectile (* (Variables|/Script/Engine.MovementComponent|GetVelocity _projectile) 5)))))

(event Collision|EventHit
  (params (MyComp :type Primitive%20Component%20Object%20Reference) (Other :type Actor%20Object%20Reference) (OtherComp :type Primitive%20Component%20Object%20Reference) (bSelfMoved :type Boolean) (HitLocation :type Vector :default "0, 0, 0") (HitNormal :type Vector :default "0, 0, 0") (NormalImpulse :type Vector :default "0, 0, 0") (Hit :type Hit%20Result%20Structure%20%28by%20ref%29))
  ;[1 1 1] Destroy on hit
  (Actor|DestroyActor))

(fn ConstructionScript)