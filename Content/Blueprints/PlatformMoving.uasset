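; Moving platform that slides along a configurable axis via a timeline, starting at play when a non-visible Timer widget exists, or via TriggerMove if trigger-driven.
; Overlapping blue or red force fields doubles or halves the timeline play rate, restored when the overlap ends.
; An optional auto-destruct mode applies a distinct neon material and destroys the platform after a delay once the first-person character hits it.
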(event OnComponentHit(Cube)
  (params (HitComponent :type Primitive%20Component%20Object%20Reference) (OtherActor :type Actor%20Object%20Reference) (OtherComp :type Primitive%20Component%20Object%20Reference) (NormalImpulse :type Vector :default "0, 0, 0") (Hit :type Hit%20Result%20Structure%20%28by%20ref%29))
  ;[1 1 1] ForceField Detection
  (if (Variables|Default|GetIsAutoDestructing)
    (Utilities|Casting|CastToFirstPersonCharacter OtherActor)
    (Utilities|FlowControl|Delay (Variables|Default|GetDestructionDelay))
    (Actor|DestroyActor)))

(event OnComponentBeginOverlap(Cube)
  (params (OverlappedComponent :type Primitive%20Component%20Object%20Reference) (OtherActor :type Actor%20Object%20Reference) (OtherComp :type Primitive%20Component%20Object%20Reference) (OtherBodyIndex :type Integer) (bFromSweep :type Boolean) (SweepResult :type Hit%20Result%20Structure%20%28by%20ref%29))
  ;[1 1 1] ForceField Detection
  (Utilities|Casting|CastToForceFieldBlue OtherActor
    (:then
      (bind _output_get (Variables|Default|SetPlayRateCurrent (* (Variables|Default|GetPlayRateDefaut) 2.0)))
      (Components|Timeline|SetPlayRate (Variables|Default|GetMoving) _output_get))
    (:CastFailed
      (Utilities|Casting|CastToForceFieldRed OtherActor)
      (bind _output_get_2 (Variables|Default|SetPlayRateCurrent (* (Variables|Default|GetPlayRateDefaut) 0.5)))
      (Components|Timeline|SetPlayRate (Variables|Default|GetMoving) _output_get_2))))

(event OnComponentEndOverlap(Cube)
  (params (OverlappedComponent :type Primitive%20Component%20Object%20Reference) (OtherActor :type Actor%20Object%20Reference) (OtherComp :type Primitive%20Component%20Object%20Reference) (OtherBodyIndex :type Integer))
  ;[1 1 1] ForceField Detection
  (Utilities|Casting|CastToForceFieldBlue OtherActor
    (:then
      _)
    (:CastFailed
      (Utilities|Casting|CastToForceFieldRed OtherActor)))
  (bind _output_get (Variables|Default|SetPlayRateCurrent (Variables|Default|GetPlayRateDefaut)))
  (Components|Timeline|SetPlayRate (Variables|Default|GetMoving) _output_get))

(event Custom|StartMoving
  ;[1 1 1] Translation
  (if (not (Variables|Default|GetIsTriggered))
    (Utilities|FlowControl|Sequence
      (:then_0
        (bind _moving (Timeline|Moving Play)
          (:Update
            (Transformation|SetRelativeLocation (Variables|Default|GetCube) (* (Math|Vector|MakeVector (* _moving (Variables|Default|GetVariation)) (* _moving (Variables|Default|GetVariation)) (* _moving (Variables|Default|GetVariation))) (Variables|Default|GetMovingAxis)) false false))))
      (:then_1
        (Components|Timeline|SetPlayRate (Variables|Default|GetMoving) (Variables|Default|GetPlayRateCurrent))))))

(event Custom|TriggerMove
  ;[1 1 1] Translation
  (Utilities|FlowControl|Sequence
    (:then_0
      (bind _moving (Timeline|Moving Play)
        (:Update
          (Transformation|SetRelativeLocation (Variables|Default|GetCube) (* (Math|Vector|MakeVector (* _moving (Variables|Default|GetVariation)) (* _moving (Variables|Default|GetVariation)) (* _moving (Variables|Default|GetVariation))) (Variables|Default|GetMovingAxis)) false false))))
    (:then_1
      (Components|Timeline|SetPlayRate (Variables|Default|GetMoving) (Variables|Default|GetPlayRateCurrent)))))

(event EventBeginPlay
  ;[1 1 1] Translation
  (Variables|Default|SetPlayRateCurrent (Variables|Default|GetPlayRateDefaut))
  (Utilities|FlowControl|Sequence
    (:then_0
      (if (Variables|Default|GetIsAutoDestructing)
        (Rendering|Material|SetMaterial (Variables|Default|GetStaticMesh) 0 "/Game/Materials/M_Neon_PlatformAutoDestructing.M_Neon_PlatformAutoDestructing")
        (Rendering|Material|SetMaterial (Variables|Default|GetStaticMesh1) 0 "/Game/Materials/M_Neon_PlatformAutoDestructing.M_Neon_PlatformAutoDestructing")
        (Rendering|Material|SetMaterial (Variables|Default|GetStaticMesh2) 0 "/Game/Materials/M_Neon_PlatformAutoDestructing.M_Neon_PlatformAutoDestructing")
        (Rendering|Material|SetMaterial (Variables|Default|GetStaticMesh3) 0 "/Game/Materials/M_Neon_PlatformAutoDestructing.M_Neon_PlatformAutoDestructing")))
    (:then_1
      (bind _foundwidgets (Widget|GetAllWidgetsOfClass "/Game/Blueprints/Timer.Timer_C" true))
      (bind _array_element (Utilities|Array|ForEachLoopwithBreak _foundwidgets)
        (:LoopBody
          (if (not (Widget|IsVisible _array_element))
            (CallFunction|StartMoving)))))))

(fn ConstructionScript)

(fn StopMoving
  (Audio|Components|Audio|Stop (Variables|Default|GetMoving)))