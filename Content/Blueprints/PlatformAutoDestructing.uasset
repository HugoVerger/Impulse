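; A moving platform that destroys itself after a configurable delay once the first-person character hits it.
; On BeginPlay it starts moving if it finds a hidden top-level Timer widget, with a timeline offsetting the cube along MovingAxis, scaled by Variation.
; Overlapping a blue force field doubles the timeline's play rate and a red one halves it, while ending any overlap restores the base rate.
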(event OnComponentHit(Cube)
  (params (HitComponent :type Primitive%20Component%20Object%20Reference) (OtherActor :type Actor%20Object%20Reference) (OtherComp :type Primitive%20Component%20Object%20Reference) (NormalImpulse :type Vector :default "0, 0, 0") (Hit :type Hit%20Result%20Structure%20%28by%20ref%29))
  ;[1 1 1] ForceField Detection
  (Utilities|Casting|CastToFirstPersonCharacter OtherActor)
  (Utilities|FlowControl|Delay (Variables|Default|GetDestructionDelay))
  (Actor|DestroyActor))

(event OnComponentBeginOverlap(Cube)
  (params (OverlappedComponent :type Primitive%20Component%20Object%20Reference) (OtherActor :type Actor%20Object%20Reference) (OtherComp :type Primitive%20Component%20Object%20Reference) (OtherBodyIndex :type Integer) (bFromSweep :type Boolean) (SweepResult :type Hit%20Result%20Structure%20%28by%20ref%29))
  ;[1 1 1] ForceField Detection
  (Utilities|Casting|CastToForceFieldBlue OtherActor
    (:then
      (Components|Timeline|SetPlayRate (Variables|Default|GetMoving) (* (Variables|Default|GetPlayRate) 2.0)))
    (:CastFailed
      (Utilities|Casting|CastToForceFieldRed OtherActor)
      (Components|Timeline|SetPlayRate (Variables|Default|GetMoving) (* (Variables|Default|GetPlayRate) 0.5)))))

(event OnComponentEndOverlap(Cube)
  (params (OverlappedComponent :type Primitive%20Component%20Object%20Reference) (OtherActor :type Actor%20Object%20Reference) (OtherComp :type Primitive%20Component%20Object%20Reference) (OtherBodyIndex :type Integer))
  ;[1 1 1] ForceField Detection
  (Components|Timeline|SetPlayRate (Variables|Default|GetMoving) (Variables|Default|GetPlayRate)))

(event Custom|StartMoving
  ;[1 1 1] Translation
  (Utilities|FlowControl|Sequence
    (:then_0
      (bind _moving (Timeline|Moving Play)
        (:Update
          (Transformation|SetRelativeLocation (Variables|Default|GetCube) (* (Math|Vector|MakeVector (* _moving (Variables|Default|GetVariation)) (* _moving (Variables|Default|GetVariation)) (* _moving (Variables|Default|GetVariation))) (Variables|Default|GetMovingAxis)) false false))))
    (:then_1
      (Components|Timeline|SetPlayRate (Variables|Default|GetMoving) (Variables|Default|GetPlayRate)))))

(event EventBeginPlay
  ;[1 1 1] Translation
  (bind _foundwidgets (Widget|GetAllWidgetsOfClass "/Game/Blueprints/Timer.Timer_C" true))
  (bind _array_element (Utilities|Array|ForEachLoopwithBreak _foundwidgets)
    (:LoopBody
      (if (not (Widget|IsVisible _array_element))
        (CallFunction|StartMoving)))))

(fn ConstructionScript)