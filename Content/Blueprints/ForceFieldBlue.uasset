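; ForceFieldBlue is a blue force field actor that deploys by expanding and can be neutralized on contact.
; On BeginPlay, a timeline drives the relative scale of its Sphere component to animate deployment.
; On overlap, it destroys itself if the other actor is a ForceFieldRed, or if that actor's static mesh uses M_Metal_Steel in its first material slot.
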(event Collision|EventActorBeginOverlap
  (params (OtherActor :type Actor%20Object%20Reference))
  (bind _returnvalue (Actor|GetComponentbyClass OtherActor "/Script/Engine.StaticMeshComponent"))
  ;[1 1 1] ForceField neutralization
  (Utilities|Casting|CastToForceFieldRed OtherActor
    (:then
      (Actor|DestroyActor :!label _label))
    (:CastFailed
      (if (Utilities|IsValid _returnvalue)
        (if (== (Rendering|Material|GetMaterial _returnvalue 0) "/Game/StarterContent/Materials/M_Metal_Steel.M_Metal_Steel")
          (goto _label))))))

(event EventBeginPlay
  ;[1 1 1] ForceField deployment
  (bind _scalertrack (Timeline|Timeline_0 PlayFromStart)
    (:Update
      (Transformation|SetRelativeScale3D (Variables|Default|GetSphere) _scalertrack))))

(fn ConstructionScript)