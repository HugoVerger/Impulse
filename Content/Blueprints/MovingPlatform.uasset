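; Moving platform Blueprint that travels along a timeline-driven path and changes speed inside force fields.
; On BeginPlay, a timeline feeds its Translator track into the Cube's relative location without sweeping.
; Cube overlaps with ForceFieldLeft double the timeline's play rate, while ForceFieldRight halves it.
; Any end overlap restores normal speed, regardless of which actor left.
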(event OnComponentBeginOverlap(Cube)
  (params (OverlappedComponent :type Primitive%20Component%20Object%20Reference) (OtherActor :type Actor%20Object%20Reference) (OtherComp :type Primitive%20Component%20Object%20Reference) (OtherBodyIndex :type Integer) (bFromSweep :type Boolean) (SweepResult :type Hit%20Result%20Structure%20%28by%20ref%29))
  ;[1 1 1] ForceField Detection
  (Utilities|Casting|CastToForceFieldLeft OtherActor
    (:then
      (Components|Timeline|SetPlayRate (Variables|Default|GetTimeline_0) 2.0))
    (:CastFailed
      (Utilities|Casting|CastToForceFieldRight OtherActor)
      (Components|Timeline|SetPlayRate (Variables|Default|GetTimeline_0) 0.5))))

(event OnComponentEndOverlap(Cube)
  (params (OverlappedComponent :type Primitive%20Component%20Object%20Reference) (OtherActor :type Actor%20Object%20Reference) (OtherComp :type Primitive%20Component%20Object%20Reference) (OtherBodyIndex :type Integer))
  ;[1 1 1] ForceField Detection
  (Components|Timeline|SetPlayRate (Variables|Default|GetTimeline_0) 1.0))

(event EventBeginPlay
  ;[1 1 1] Translation
  (bind _translator (Timeline|Timeline_0 Play)
    (:Update
      (Transformation|SetRelativeLocation (Variables|Default|GetCube) _translator false false))))

(fn ConstructionScript)