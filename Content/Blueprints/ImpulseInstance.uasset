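; Game instance that holds and persists user preferences: mouse sensitivity and inversion, player name and sound class volumes.
; On Init it loads the UserPrefSlot ImpulseSave, if present, and applies volumes through Victory sound nodes.
; Setter functions store mouse settings and push them to the current FirstPersonCharacter.
; SaveValues writes current values back, reading volumes live from the sound classes and creating the save object when none exists.
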(event EventInit
  ;[1 1 1] Loading saved user prefs and setting them as default values
  (bind _returnvalue (SaveGame|DoesSaveGameExist "UserPrefSlot"))
  (if _returnvalue
    (bind _returnvalue_2 (SaveGame|LoadGamefromSlot "UserPrefSlot"))
    (bind _asimpulse_save (Utilities|Casting|CastToImpulseSave _returnvalue_2))
    (Variables|Default|SetMouseSensibility (Variables|/Game/Blueprints/ImpulseSave.ImpulseSave_C|GetMouseSensibility _asimpulse_save))
    (Variables|Default|SetMouseInvert (Variables|/Game/Blueprints/ImpulseSave.ImpulseSave_C|GetMouseInvert _asimpulse_save))
    (Variables|Default|SetPlayerName (Variables|/Game/Blueprints/ImpulseSave.ImpulseSave_C|GetPlayerName _asimpulse_save))
    (Class|VictoryBPFunctionLibrary|VictorySoundVolumeChange "/Game/Sounds/Master.Master" (Variables|/Game/Blueprints/ImpulseSave.ImpulseSave_C|GetMasterVolume _asimpulse_save))
    (Class|VictoryBPFunctionLibrary|VictorySoundVolumeChange "/Game/Sounds/Master.Music" (Variables|/Game/Blueprints/ImpulseSave.ImpulseSave_C|GetMusicVolume _asimpulse_save))
    (Class|VictoryBPFunctionLibrary|VictorySoundVolumeChange "/Game/Sounds/Master.Ambients" (Variables|/Game/Blueprints/ImpulseSave.ImpulseSave_C|GetAmbientsVolume _asimpulse_save))
    (Class|VictoryBPFunctionLibrary|VictorySoundVolumeChange "/Game/Sounds/Master.Effects" (Variables|/Game/Blueprints/ImpulseSave.ImpulseSave_C|GetEffectsVolume _asimpulse_save))
    (Class|VictoryBPFunctionLibrary|VictorySoundVolumeChange "/Game/Sounds/Master.Voices" (Variables|/Game/Blueprints/ImpulseSave.ImpulseSave_C|GetVoicesVolume _asimpulse_save))))

(fn ChangeMouseSensibility
  (params (mouseSens :type Float%20%28single-precision%29))
  (bind _output_get (Variables|Default|SetMouseSensibility mouseSens))
  (bind _asfirst_person_character (Utilities|Casting|CastToFirstPersonCharacter (Game|GetPlayerCharacter 0)))
  (Variables|/Game/Blueprints/FirstPersonCharacter.FirstPersonCharacter_C|SetSensitivity _asfirst_person_character _output_get))

(fn ChangeMouseInvert
  (params (invert :type Boolean))
  (bind _output_get (Variables|Default|SetMouseInvert invert))
  (bind _asfirst_person_character (Utilities|Casting|CastToFirstPersonCharacter (Game|GetPlayerCharacter 0)))
  (Variables|/Game/Blueprints/FirstPersonCharacter.FirstPersonCharacter_C|SetInvert _asfirst_person_character _output_get))

(fn SaveValues
  (bind _returnvalue (Class|VictoryBPFunctionLibrary|VictoryGetSoundVolume "/Game/Sounds/Master.Voices"))
  (bind _returnvalue_2 (Class|VictoryBPFunctionLibrary|VictoryGetSoundVolume "/Game/Sounds/Master.Master"))
  (bind _returnvalue_3 (Class|VictoryBPFunctionLibrary|VictoryGetSoundVolume "/Game/Sounds/Master.Music"))
  (bind _returnvalue_4 (Class|VictoryBPFunctionLibrary|VictoryGetSoundVolume "/Game/Sounds/Master.Ambients"))
  (bind _returnvalue_5 (Class|VictoryBPFunctionLibrary|VictoryGetSoundVolume "/Game/Sounds/Master.Effects"))
  ;[1 1 1] Saving current user pref values to disk
  (bind _returnvalue_6 (SaveGame|DoesSaveGameExist "UserPrefSlot"))
  (if _returnvalue_6
    (bind _returnvalue_7 (SaveGame|LoadGamefromSlot "UserPrefSlot"))
    (bind _asimpulse_save (Utilities|Casting|CastToImpulseSave _returnvalue_7))
    (Variables|/Game/Blueprints/ImpulseSave.ImpulseSave_C|SetMouseSensibility _asimpulse_save (Variables|Default|GetMouseSensibility))
    (Variables|/Game/Blueprints/ImpulseSave.ImpulseSave_C|SetMouseInvert _asimpulse_save (Variables|Default|GetMouseInvert))
    (Variables|/Game/Blueprints/ImpulseSave.ImpulseSave_C|SetMasterVolume _asimpulse_save _returnvalue_2)
    (Variables|/Game/Blueprints/ImpulseSave.ImpulseSave_C|SetMusicVolume _asimpulse_save _returnvalue_3)
    (Variables|/Game/Blueprints/ImpulseSave.ImpulseSave_C|SetAmbientsVolume _asimpulse_save _returnvalue_4)
    (Variables|/Game/Blueprints/ImpulseSave.ImpulseSave_C|SetEffectsVolume _asimpulse_save _returnvalue_5)
    (Variables|/Game/Blueprints/ImpulseSave.ImpulseSave_C|SetVoicesVolume _asimpulse_save _returnvalue)
    (Variables|/Game/Blueprints/ImpulseSave.ImpulseSave_C|SetPlayerName _asimpulse_save (Variables|Default|GetPlayerName))
    (SaveGame|SaveGametoSlot _asimpulse_save "UserPrefSlot")
    (else
      (bind _returnvalue_8 (SaveGame|CreateSaveGameObject "/Game/Blueprints/ImpulseSave.ImpulseSave_C"))
      (bind _asimpulse_save_2 (Utilities|Casting|CastToImpulseSave _returnvalue_8))
      (Variables|/Game/Blueprints/ImpulseSave.ImpulseSave_C|SetMouseSensibility _asimpulse_save_2 (Variables|Default|GetMouseSensibility))
      (Variables|/Game/Blueprints/ImpulseSave.ImpulseSave_C|SetMouseInvert _asimpulse_save_2 (Variables|Default|GetMouseInvert))
      (Variables|/Game/Blueprints/ImpulseSave.ImpulseSave_C|SetMasterVolume _asimpulse_save_2 _returnvalue_2)
      (Variables|/Game/Blueprints/ImpulseSave.ImpulseSave_C|SetMusicVolume _asimpulse_save_2 _returnvalue_3)
      (Variables|/Game/Blueprints/ImpulseSave.ImpulseSave_C|SetAmbientsVolume _asimpulse_save_2 _returnvalue_4)
      (Variables|/Game/Blueprints/ImpulseSave.ImpulseSave_C|SetEffectsVolume _asimpulse_save_2 _returnvalue_5)
      (Variables|/Game/Blueprints/ImpulseSave.ImpulseSave_C|SetVoicesVolume _asimpulse_save_2 _returnvalue)
      (Variables|/Game/Blueprints/ImpulseSave.ImpulseSave_C|SetPlayerName _asimpulse_save_2 (Variables|Default|GetPlayerName))
      (SaveGame|SaveGametoSlot _asimpulse_save_2 "UserPrefSlot"))))