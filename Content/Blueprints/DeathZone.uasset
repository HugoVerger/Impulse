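; DeathZone is a trigger volume that kills the first-person player on contact and restarts the level.
; When a FirstPersonCharacter overlaps its box, it spawns an explosion at the character and applies a red camera fade that holds when finished.
; After a short delay it destroys the character, prints a death message and reopens the current level by name.
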(event OnComponentBeginOverlap(Box)
  (params (OverlappedComponent :type Primitive%20Component%20Object%20Reference) (OtherActor :type Actor%20Object%20Reference) (OtherComp :type Primitive%20Component%20Object%20Reference) (OtherBodyIndex :type Integer) (bFromSweep :type Boolean) (SweepResult :type Hit%20Result%20Structure%20%28by%20ref%29))
  ;[1 1 1] DeathZone
  (bind _asfirst_person_character (Utilities|Casting|CastToFirstPersonCharacter OtherActor))
  (Effects|SpawnEmitteratLocation "/Game/StarterContent/Particles/P_Explosion.P_Explosion" (Transformation|GetActorLocation _asfirst_person_character))
  (CameraFades|StartCameraFade (Game|GetPlayerCameraManager 0) 0.6 0.2 0.4 "(R=1.000000,G=0.000000,B=0.000000,A=1.000000)" false true)
  (Utilities|FlowControl|Delay 0.3)
  (Actor|DestroyActor _asfirst_person_character)
  (Development|PrintString "YOU DIED !" true true "(R=1.000000,G=0.000000,B=0.000000,A=1.000000)")
  (bind _returnvalue (Game|GetCurrentLevelName true))
  (Game|OpenLevel(byName) (Utilities|String|StringToName _returnvalue)))

(fn ConstructionScript)