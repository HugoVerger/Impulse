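; DoorBig is a sliding door that opens when the first-person character enters its trigger box and closes when they leave.
; Box overlaps play and reverse the DoorPosition timeline, whose DoorSlider track sets the Cube's relative location.
; The LockedDoor flag blocks both responses.
; An opening sound plays at the door with attenuation, scaled by master and effects volume from ImpulseInstance, while closing is silent.
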(event OnComponentBeginOverlap(Box)
  (params (OverlappedComponent :type Primitive%20Component%20Object%20Reference) (OtherActor :type Actor%20Object%20Reference) (OtherComp :type Primitive%20Component%20Object%20Reference) (OtherBodyIndex :type Integer) (bFromSweep :type Boolean) (SweepResult :type Hit%20Result%20Structure%20%28by%20ref%29))
  ;[1 1 1] Door opening and closing
  (if (not (Variables|Default|GetLockedDoor))
    (Utilities|Casting|CastToFirstPersonCharacter OtherActor)
    (bind _asimpulse_instance (Utilities|Casting|CastToImpulseInstance (Game|GetGameInstance)))
    (Audio|PlaySoundatLocation "/Game/Sounds/DoorOpening.DoorOpening" (Transformation|GetActorLocation) "0, 0, 0" (* (Variables|/Game/Blueprints/ImpulseInstance.ImpulseInstance_C|GetMasterVolume _asimpulse_instance) (Variables|/Game/Blueprints/ImpulseInstance.ImpulseInstance_C|GetEffectsVolume _asimpulse_instance)) 1.0 0.0 "/Game/Sounds/SoundAttenuation.SoundAttenuation")
    (bind _doorslider (Timeline|DoorPosition Play)
      (:Update
        (Transformation|SetRelativeLocation (Variables|Default|GetCube) _doorslider false false)))))

(event OnComponentEndOverlap(Box)
  (params (OverlappedComponent :type Primitive%20Component%20Object%20Reference) (OtherActor :type Actor%20Object%20Reference) (OtherComp :type Primitive%20Component%20Object%20Reference) (OtherBodyIndex :type Integer))
  ;[1 1 1] Door opening and closing
  (if (not (Variables|Default|GetLockedDoor))
    (Utilities|Casting|CastToFirstPersonCharacter OtherActor)
    (bind _doorslider (Timeline|DoorPosition Reverse)
      (:Update
        (Transformation|SetRelativeLocation (Variables|Default|GetCube) _doorslider false false)))))

(fn ConstructionScript)