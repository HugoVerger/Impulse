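; Red force field actor that deploys in the world and can be neutralized by a blue force field.
; On BeginPlay it plays a deploy sound while a timeline animates the sphere's scale.
; Overlapping a ForceFieldBlue destroys it only if the player's last shot was blue, as tracked on FirstPersonCharacter.
; Destruction spawns a red repulsion particle effect and sound, with both sounds scaled by the ImpulseInstance volume settings.
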(event EventDestroyed
  ;[1 1 1] Destruction Effect
  (Effects|SpawnEmitteratLocation "/Game/Particles/RepulsionRed.RepulsionRed" (Transformation|GetActorLocation))
  (bind _asimpulse_instance (Utilities|Casting|CastToImpulseInstance (Game|GetGameInstance)))
  (Audio|PlaySoundatLocation "/Game/Sounds/FF_destroy.FF_destroy" (Transformation|GetActorLocation) "0, 0, 0" (* (Variables|/Game/Blueprints/ImpulseInstance.ImpulseInstance_C|GetMasterVolume _asimpulse_instance) (Variables|/Game/Blueprints/ImpulseInstance.ImpulseInstance_C|GetEffectsVolume _asimpulse_instance)) 1.0 0.0 "/Game/Sounds/SoundAttenuation.SoundAttenuation"))

(event Collision|EventActorBeginOverlap
  (params (OtherActor :type Actor%20Object%20Reference))
  ;[1 1 1] ForceField neutralization
  (Utilities|Casting|CastToForceFieldBlue OtherActor)
  (bind _asfirst_person_character (Utilities|Casting|CastToFirstPersonCharacter (Game|GetPlayerCharacter 0)))
  (if (Variables|/Game/Blueprints/FirstPersonCharacter.FirstPersonCharacter_C|GetIsBlueLastShooted _asfirst_person_character)
    (Actor|DestroyActor)))

(event EventBeginPlay
  ;[1 1 1] ForceField deployment
  (bind _asimpulse_instance (Utilities|Casting|CastToImpulseInstance (Game|GetGameInstance)))
  (Audio|PlaySoundatLocation "/Game/Sounds/FF_deploy.FF_deploy" (Transformation|GetActorLocation) "0, 0, 0" (* (Variables|/Game/Blueprints/ImpulseInstance.ImpulseInstance_C|GetMasterVolume _asimpulse_instance) (Variables|/Game/Blueprints/ImpulseInstance.ImpulseInstance_C|GetEffectsVolume _asimpulse_instance)) 1.0 0.0 "/Game/Sounds/SoundAttenuation.SoundAttenuation")
  (bind _scalertrack (Timeline|Timeline_0 PlayFromStart)
    (:Update
      (Transformation|SetRelativeScale3D (Variables|Default|GetSphere) _scalertrack))))

(fn ConstructionScript)