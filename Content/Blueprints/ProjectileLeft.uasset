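; Left projectile that replaces any existing ForceFieldLeft actors with a new one at its impact point, then destroys itself.
; On Hit it destroys all ForceFieldLeft actors and spawns the replacement at the hit location.
; If the hit component is a static mesh, it adds a scene component to the hit actor as an anchor, attaching it to the mesh and the force field to it.
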(event Collision|EventHit
  (params (MyComp :type Primitive%20Component%20Object%20Reference) (Other :type Actor%20Object%20Reference) (OtherComp :type Primitive%20Component%20Object%20Reference) (bSelfMoved :type Boolean) (HitLocation :type Vector) (HitNormal :type Vector :default "0, 0, 0") (NormalImpulse :type Vector :default "0, 0, 0") (Hit :type Hit%20Result%20Structure%20%28by%20ref%29))
  (bind _returnvalue (Math|Transform|MakeTransform HitLocation))
  ;[1 1 1] Spawning ForceField on hit then destroying projectile
  (bind _outactors (Actor|GetAllActorsOfClass "/Game/Blueprints/ForceFieldLeft.ForceFieldLeft_C"))
  (Actor|DestroyActor _outactors)
  (bind _returnvalue_2 (Game|SpawnActorfromClass "/Game/Blueprints/ForceFieldLeft.ForceFieldLeft_C" _returnvalue "AlwaysSpawn" 0 0)) ; Spawn projectile
  (Utilities|Casting|CastToStaticMeshComponent OtherComp
    (:then
      (bind _returnvalue_3 (AddComponent|AddSceneComponent Other false (Math|Transform|MakeTransform (Math|Transform|InverseTransformLocation (Class|KismetMathLibrary|ConvertTransformtoRelative _returnvalue (Transformation|GetWorldTransform OtherComp)) "0, 0, 0"))))
      (Transformation|AttachComponentToComponent _returnvalue_3 OtherComp "None" "KeepRelative" "KeepWorld" "KeepWorld" false)
      (Transformation|AttachComponentToComponent _returnvalue_2 _returnvalue_3 "None" "SnapToTarget" "KeepWorld" "KeepWorld" false))
    (:CastFailed
      _))
  (Actor|DestroyActor))

(fn ConstructionScript)