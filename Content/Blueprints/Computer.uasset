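; Interactable computer actor that opens a ComputerMenu widget when the player presses Use nearby.
; On begin play it reads the Use key binding and shows a "press to use" prompt on its TextRender.
; A sphere overlap tracks whether the FirstPersonCharacter is inside.
; Use then plays a click, switches to UI-only input with a cursor, blurs the camera via depth-of-field settings, and pauses the game after a short delay.
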(event OnComponentBeginOverlap(Sphere)
  (params (OverlappedComponent :type Primitive%20Component%20Object%20Reference) (OtherActor :type Actor%20Object%20Reference) (OtherComp :type Primitive%20Component%20Object%20Reference) (OtherBodyIndex :type Integer) (bFromSweep :type Boolean) (SweepResult :type Hit%20Result%20Structure%20%28by%20ref%29))
  ;[1 1 1] Trigger to tell if the player is close enough to detect use key
  (Utilities|Casting|CastToFirstPersonCharacter OtherActor)
  (Variables|Default|SetIsPlayerInside true))

(event OnComponentEndOverlap(Sphere)
  (params (OverlappedComponent :type Primitive%20Component%20Object%20Reference) (OtherActor :type Actor%20Object%20Reference) (OtherComp :type Primitive%20Component%20Object%20Reference) (OtherBodyIndex :type Integer))
  ;[1 1 1] Trigger to tell if the player is close enough to detect use key
  (Utilities|Casting|CastToFirstPersonCharacter OtherActor)
  (Variables|Default|SetIsPlayerInside false))

(event EventBeginPlay
  ;[1 1 1] Enable and display the key to press
  (Input|EnableInput (Game|GetPlayerController 0))
  (bind _array_element (Utilities|Array|ForEachLoopwithBreak (Class|VictoryBPFunctionLibrary|VictoryGetAllActionKeyBindings) :!label _label)
    (:LoopBody
      (if (Utilities|Enum|Equal(Enum) (.ActionName (Utilities|Struct|BreakVictoryInput _array_element)) "Use")
        (Rendering|Components|TextRender|SetText (Variables|Default|GetTextRender) (Utilities|Text|ToText(String) (Utilities|String|Append "Press " (Utilities|String|ToString(Text) (Class|KismetInputLibrary|KeyGetDisplayName (.Key (Utilities|Struct|BreakVictoryInput _array_element)))) " to use !")))
        (goto _label Break)))))

(event Input|ActionEvents|InputActionUse
  (params (Key :type Key%20Structure :default "AnyKey"))
  (bind _returnvalue (Game|GetPlayerController 0))
  ;[1 1 1] Use Input
  (:Pressed
    (if (Variables|Default|GetIsPlayerInside)
      (Audio|PlaySoundatLocation "/Game/MenuAssets/SciFiClick.SciFiClick" (Transformation|GetActorLocation))
      (bind _returnvalue_2 (UserInterface|CreateWidget "/Game/Blueprints/Menus/ComputerMenu.ComputerMenu_C"))
      (UserInterface|Viewport|AddtoViewport _returnvalue_2 0)
      (Variables|/Script/Engine.PlayerController|SetbShowMouseCursor _returnvalue true)
      (Input|SetInputModeUIOnly _returnvalue _returnvalue_2 "DoNotLock")
      (bind _asfirst_person_character (Utilities|Casting|CastToFirstPersonCharacter (Game|GetPlayerCharacter 0)))
      (Utilities|Struct|SetmembersinPostProcessSettings (Variables|/Script/Engine.CameraComponent|GetPostProcessSettings (Variables|/Game/Blueprints/FirstPersonCharacter.FirstPersonCharacter_C|GetFirstPersonCamera _asfirst_person_character)) "DOFM_Gaussian" 1e+04)
      (Utilities|FlowControl|Delay 0.15)
      (Game|SetGamePaused true))))

(fn ConstructionScript)