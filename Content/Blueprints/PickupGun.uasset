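; PickupGun is a gun pickup actor that spins in place until the first-person character walks over it.
; Tick rotates the gun around yaw at a constant rate scaled by delta time.
; On overlap with a FirstPersonCharacter, it reveals that character's Mesh2P and its children, shows the HUD widget, then destroys itself.
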(event Collision|EventActorBeginOverlap
  (params (OtherActor :type Actor%20Object%20Reference))
  ;[1 1 1] Displaying HUD and gun on pickup
  (bind _asfirst_person_character (Utilities|Casting|CastToFirstPersonCharacter OtherActor))
  (Rendering|SetVisibility (Variables|/Game/Blueprints/FirstPersonCharacter.FirstPersonCharacter_C|GetMesh2P _asfirst_person_character) true true)
  (Widget|SetVisibility (Variables|/Game/Blueprints/FirstPersonCharacter.FirstPersonCharacter_C|GetHUD_Reference _asfirst_person_character) "Visible")
  (Actor|DestroyActor))

(event EventTick
  (params (DeltaSeconds :type Float%20%28single-precision%29))
  ;[1 1 1] Rotation
  (Transformation|AddLocalRotation (Variables|Default|GetPickupGun) (Math|Rotator|MakeRotator 0.0 0.0 (* DeltaSeconds -2e+02)) false false))

(fn ConstructionScript)